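; BP_Avatar is a player character that turns to face the mouse cursor and wears a data-driven costume.
; On BeginPlay, clothing meshes follow the main mesh's pose, and after a short delay a DT_Costumes row sets its material.
; Each tick, the locally controlled avatar yaws toward the cursor hit point and sends that rotation through ServerSetRotation.
; OnDeath disables movement, notifies ASGameMode, then hides the actor and disables collision.
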(event `self.ReceiveBeginPlay`
  (bind _mesh (`self.Mesh`))
  (`SkinnedMeshComponent.SetLeaderPoseComponent` (`self.SK_Pants_014`) _mesh false false)
  (`SkinnedMeshComponent.SetLeaderPoseComponent` (`self.HatMesh `) _mesh false false)
  (`SkinnedMeshComponent.SetLeaderPoseComponent` (`self.SK_Shoe_Sneakers_009`) _mesh false false)
  (set `CharacterMovementComponent.bOrientRotationToMovement` false (`self.CharacterMovement`))
  (bind _asasplayer_controller (cast `ASPlayerController` (`self.GetController`)))
  (`WidgetBlueprintLibrary.SetInputMode_GameOnly` _asasplayer_controller)
  (set `PlayerController.bShowMouseCursor` false _asasplayer_controller)
  (`KismetSystemLibrary.Delay` 0.2)
  (`self.Apply Costume From Player State`))

(event `self.ReceiveTick`
  (params (DeltaSeconds :type "Float (single-precision)"))
  (bind _returnvalue (`KismetMathLibrary.MakeRotator` 0.0 0.0 (.yaw (`KismetMathLibrary.FindLookAtRotation` (`self.K2_GetActorLocation`) (`.Location` (`GameplayStatics.BreakHitResult` (`PlayerController.GetHitResultUnderCursorByChannel` (`GameplayStatics.GetPlayerController` 0) "TraceTypeQuery1" true)))))))
  (if (`self.IsLocallyControlled`)
    (`self.K2_SetActorRotation` _returnvalue)
    (`self.Server_SetRotation` _returnvalue)))

(event `self.OnDeath`
  (set `self.bIsDead` true)
  (`CharacterMovementComponent.DisableMovement` (`self.CharacterMovement`))
  (bind _asasgame_mode (cast `ASGameMode` (`GameplayStatics.GetGameMode`)))
  (bind _asplayer_controller (cast `PlayerController` (`self.GetController`)))
  (`ASGameMode.OnPlayerDied` _asasgame_mode _asplayer_controller)
  (`self.SetActorHiddenInGame` true)
  (`self.SetActorEnableCollision` false))

(event `Apply Costume From Player State`
  (bind _returnvalue (`|GetDataTableRow` "/Game/Blueprints/DT_Costumes.DT_Costumes" (`self.ReplicatedCostumeRowName`))
    (:`then`
      (`PrimitiveComponent.SetMaterial` (`self.Mesh`) 0 (`.CostumeMaterial_6_90F32C7D44A6F0EFC79EEF8A66542614` (break `/Game/Blueprints/S_CostumeData` _returnvalue))))))

(fn `UserConstructionScript`)