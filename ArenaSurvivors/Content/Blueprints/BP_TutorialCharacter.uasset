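; BP_TutorialCharacter is a character with modular clothing and a pause key, apparently for the tutorial.
; On BeginPlay the pants, hat and sneaker meshes take the main Mesh as leader pose component, so they follow its animation.
; Pressing Escape on the locally controlled character adds a W_PauseMenu widget, pauses the game, shows the cursor and switches input to UI only.
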(event `self.ReceiveBeginPlay`
  (bind _mesh (`self.Mesh`))
  (`SkinnedMeshComponent.SetLeaderPoseComponent` (`self.SK_Pants_014`) _mesh false false)
  (`SkinnedMeshComponent.SetLeaderPoseComponent` (`self.HatMesh `) _mesh false false)
  (`SkinnedMeshComponent.SetLeaderPoseComponent` (`self.SK_Shoe_Sneakers_009`) _mesh false false))

(event `Key|Escape`
  (params (Key :type "Key Structure"))
  (bind _returnvalue (`GameplayStatics.GetPlayerController` 0))
  (:`Pressed`
    (if (`self.IsLocallyControlled`)
      (bind _returnvalue_2 (`|CreateWidget` "/Game/Widgets/W_PauseMenu.W_PauseMenu_C"))
      (`UserWidget.AddToViewport` _returnvalue_2 0)
      (`GameplayStatics.SetGamePaused` true)
      (set `PlayerController.bShowMouseCursor` true _returnvalue)
      (`WidgetBlueprintLibrary.SetInputMode_UIOnlyEx` _returnvalue null))))

(fn `UserConstructionScript`)