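; Game state Blueprint that handles the end of a team match and its result message.
; OnVictory walks the player array, telling Red team avatars they won and Blue ones they lost, with the winning team hard-coded.
; It then shows a results widget whose text depends on the first local player's team.
; OnRestart removes that widget from the screen.
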(event `self.OnVictory`
  (for _array_element (`self.PlayerArray`)
    (bind _asnet_player_state (cast `NetPlayerState` _array_element))
    (bind _asbp_net_avatar (cast `/Game/Blueprints/BP_NetAvatar` (`PlayerState.PawnPrivate` _asnet_player_state)))
    (switch `EPlayerTeam` (`NetPlayerState.TeamID` _asnet_player_state)
      (:`TEAM_Blue`
        (`/Game/Blueprints/BP_NetAvatar.OnPlayerLost` _asbp_net_avatar))
      (:`TEAM_Red`
        (`/Game/Blueprints/BP_NetAvatar.OnPlayerWon` _asbp_net_avatar))))
  (`self. Show Result Message`))

(event `self.OnRestart`
  (`Widget.RemoveFromParent` (`self.Message Widget`)))

(event `Show Result Message`
  (bind _asnet_player_state (cast `NetPlayerState` (`Controller.PlayerState` (`GameplayStatics.GetPlayerController` 0))))
  (bind _returnvalue (`self.GetPlayerStateByIndex` (`self.WinningPlayer`)))
  (bind _returnvalue_2 (`|CreateWidget` "/Game/Blueprints/UMG/W_GameResults.W_GameResults_C" null (select `bool` (`|EnumEquality` (`.TeamID` (break `SPlayerInfo` (`NetPlayerState.Data` _asnet_player_state))) "TEAM_Blue") :`false` (`|FormatText` "{Name} WINS!" _) :`true` "YOU LOSE!")))
  (`UserWidget.AddToViewport` _returnvalue_2 0)
  (set `self.Message Widget` _returnvalue_2))

(fn `UserConstructionScript`)